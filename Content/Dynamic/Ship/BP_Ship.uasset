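; Player-controlled physics ship driven by thrust, yaw, pitch and roll axis inputs applied as force and torque to a Sphere component.
; Each tick shows RCS thruster effects matching rotation input, or opposing residual spin when input is zero, and lengthens the spring arm with speed.
; It also tracks acceleration, creates the ship UI on BeginPlay, and draws or prints velocity and controller motion-sensor debug data.
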(event EventBeginPlay
  (|SetDefaultCameraArmLenght)
  (|CreateShipUI
    (:NewParam
      (|SetPLayerController))))

(event EventTick
  (params (DeltaSeconds :type Float%20%28single-precision%29))
  (Rendering|Debug|DrawDebugArrow
    (:NewParam
      (|UpdateInputs)
      (|UpdateCrosshair)
      (|ShowRCS
        (:then_3
          (|UpdateAcceleration DeltaSeconds)
          (|UpdateArmLag)
          (|Move
            (:NewParam
              (|Rotate))))))))

(event Input|AxisEvents|InputAxisAccelerate
  (params (AxisValue :type Float%20%28single-precision%29))
  (Variables|Default|SetThrust%20Input AxisValue))

(event Input|AxisEvents|InputAxisYaw
  (params (AxisValue :type Float%20%28single-precision%29))
  (Variables|Default|SetYaw%20Input AxisValue))

(event Input|AxisEvents|InputAxisPitch
  (params (AxisValue :type Float%20%28single-precision%29))
  (Variables|Default|SetPitch%20Input AxisValue))

(event Input|AxisEvents|InputAxisRoll
  (params (AxisValue :type Float%20%28single-precision%29))
  (Variables|Default|SetRoll%20Input AxisValue))

(fn ConstructionScript)

(fn SetRCSState
  (params (RCS :type Integer) (New%20State :type Boolean))
  (switch int RCS ; 0-up 1-down 2-left 3-right 4-roll left 5-roll right
    (:0
      (Rendering|SetVisibility (Variables|Default|GetRCS%20pitch%20backward) New%20State false))
    (:1
      (Rendering|SetVisibility (Variables|Default|GetRCS%20pitch%20forward) New%20State false))
    (:2
      (Rendering|SetVisibility (Variables|Default|GetRCS%20yaw%20left) New%20State false))
    (:3
      (Rendering|SetVisibility (Variables|Default|GetRCS%20yaw%20right) New%20State false))
    (:4
      (Rendering|SetVisibility (Variables|Default|GetRCS%20roll%20left) New%20State false))
    (:5
      (Rendering|SetVisibility (Variables|Default|GetRCS%20roll%20right) New%20State false))))